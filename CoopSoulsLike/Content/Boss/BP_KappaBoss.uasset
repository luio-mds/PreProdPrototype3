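; Kappa boss character that supplies the visual side of the fight: attack animations, death and lock-on display.
; Separate events play montages for swipe, belly flop, slam and spit attacks, with no attack logic in this graph.
; It is always targetable and forwards lock-on visibility to its widget.
; Death stops movement, starts a montage, destroys the actor without waiting, then shows the win screen and pauses the game.
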(event Custom|PlaySwipeAnimation
  (Animation|Montage|PlayMontage (Variables|Character|GetMesh) "/Game/Assets/Enemies/Bosses/Kappa/Animations/AM_Kappa_ClawSwipe.AM_Kappa_ClawSwipe" 1.0 0.0 "None" false))

(event Custom|PlayBellyFlopAnimation
  (Animation|Montage|PlayMontage (Variables|Character|GetMesh) "/Game/Assets/Enemies/Bosses/Kappa/Animations/AM_KappaBellyFlop.AM_KappaBellyFlop" 1.0 0.0 "None" false))

(event Custom|PlaySlamAnimation
  (Animation|Montage|PlayMontage (Variables|Character|GetMesh) "/Game/Assets/Enemies/Bosses/Kappa/Animations/AM_Kappa_OverheadSlam.AM_Kappa_OverheadSlam" 1.0 0.0 "None" false))

(event Custom|PlaySpitAnimation
  (Animation|Montage|PlayMontage (Variables|Character|GetMesh) "/Game/Assets/Enemies/Bosses/Kappa/Animations/AM_Kappa_WaterSpit.AM_Kappa_WaterSpit" 1.0 0.0 "None" false))

(event EventLockonWidget
  (params (Visibility :type ESlateVisibility%20Enum :default "Visible"))
  (Class|BPILockon|LockonWidget(Message) (UserInterface|GetUserWidgetObject (Variables|Default|GetLockOnWidget_0)) Visibility))

(event EventOnDeathVisuals
  (Development|PrintString "KAPPA IS DEAD")
  (AI|Navigation|StopMovement (Pawn|GetController))
  (Animation|PlayAnimMontage "/Game/Assets/Enemies/Bosses/Kappa/Animations/AM_Kappa_Death.AM_Kappa_Death" 1.0 "None")
  (Actor|DestroyActor)
  (bind _returnvalue (UserInterface|CreateWidget "/Game/UI/WBP_WinScreen.WBP_WinScreen_C"))
  (UserInterface|Viewport|AddtoViewport _returnvalue 0)
  (Game|SetGamePaused true))

(fn ConstructionScript)

(fn CanbeTarget
  (return true))