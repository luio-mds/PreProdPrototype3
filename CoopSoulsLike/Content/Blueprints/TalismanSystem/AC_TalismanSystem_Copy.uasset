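; Talisman system component that keeps a talisman-to-quantity inventory map and applies passive talisman effects to the host player's samurai character.
; On BeginPlay, ApplyPassives grants damage or defense buffs, or starts looping timer health regen, for usable in-hand talismans of one use type.
; Helpers add, remove and query counts, though removal subtracts the stored count from the requested quantity.
; DrawRandom is an empty stub, and key 1 prints updated damage for debugging.
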(event Custom|ApplyPassives
  ;[1 0 1 0.502] Replicated / server
  ;;[1 0.0228 0.2776 0.5] NOTE: can be called at start of combat, for now is set with pressing 1
  (bind _keypin (Utilities|Map|ForEachLoop(Map) (Variables|Default|GetTalismanContent))
    (:then
      (if (Variables|/Game/Blueprints/TalismanSystem/TalismanData/PDA_Talisman.PDA_Talisman_C|GetCanUse? _keypin)
        (if (and (Variables|/Game/Blueprints/TalismanSystem/TalismanData/PDA_Talisman.PDA_Talisman_C|GetInHand? _keypin) (Utilities|Enum|Equal(Enum) (Variables|/Game/Blueprints/TalismanSystem/TalismanData/PDA_Talisman.PDA_Talisman_C|GetUseType _keypin) "NewEnumerator1"))
          (Development|PrintString (Utilities|String|Append "Passive Applied: " (Utilities|String|EnumtoString (Variables|/Game/Blueprints/TalismanSystem/TalismanData/PDA_Talisman.PDA_Talisman_C|GetAbility _keypin))))
          (Variables|/Game/Blueprints/TalismanSystem/TalismanData/PDA_Talisman.PDA_Talisman_C|SetCanUse? _keypin false)
          (Utilities|FlowControl|Sequence
            (:then_0
              (if (Utilities|Enum|Equal(Enum) (Variables|/Game/Blueprints/TalismanSystem/TalismanData/PDA_Talisman.PDA_Talisman_C|GetAbility _keypin) "NewEnumerator5")
                (Default|GivePlayerBuffDamage (Variables|Default|GetSamuraiCharacter) 5e+01 1e+02)))
            (:then_1
              (if (Utilities|Enum|Equal(Enum) (Variables|/Game/Blueprints/TalismanSystem/TalismanData/PDA_Talisman.PDA_Talisman_C|GetAbility _keypin) "NewEnumerator4")
                (Default|GivePlayerBuffDefense (Variables|Default|GetSamuraiCharacter) 5e+01 1e+02)))
            (:then_2
              (if (Utilities|Enum|Equal(Enum) (Variables|/Game/Blueprints/TalismanSystem/TalismanData/PDA_Talisman.PDA_Talisman_C|GetAbility _keypin) "NewEnumerator3")
                (bind _returnvalue (Utilities|Time|SetTimerbyEvent (delegate Custom|RegenerateHealth) 0.5 true))
                (Variables|Default|SetStopRegen _returnvalue)))))))))

(event Custom|DrawRandom
  ;[0.15 0.15 0.15 0.5] output is the random talisman
)

(event Custom|RegenerateHealth
  (bind _samuraicharacter (Variables|Default|GetSamuraiCharacter))
  (if (< (Variables|/Game/ThirdPerson/Blueprints/BP_ThirdPersonCharacter.BP_ThirdPersonCharacter_C|GetPlayerHealth _samuraicharacter) 1e+02)
    (Variables|/Game/ThirdPerson/Blueprints/BP_ThirdPersonCharacter.BP_ThirdPersonCharacter_C|SetPlayerHealth _samuraicharacter (Math|Float|Clamp(Float) (+ (Variables|/Game/ThirdPerson/Blueprints/BP_ThirdPersonCharacter.BP_ThirdPersonCharacter_C|GetPlayerHealth _samuraicharacter) 1e+01) 0.0 1e+02))
    (Development|PrintString (Utilities|String|ToString(Float) (Variables|/Game/ThirdPerson/Blueprints/BP_ThirdPersonCharacter.BP_ThirdPersonCharacter_C|GetPlayerHealth _samuraicharacter)))
    (else
      (Utilities|Time|ClearandInvalidateTimerbyHandle (Variables|Default|GetStopRegen)))))

(event EventBeginPlay
  (bind _asbp_network_game_mode (Utilities|Casting|CastToBP_NetworkGameMode (Game|GetGameMode)))
  (Variables|Default|SetSamuraiCharacter (Variables|/Game/ThirdPerson/Blueprints/BP_NetworkGameMode.BP_NetworkGameMode_C|GetHostPlayerCharacter _asbp_network_game_mode))
  (CallFunction|ApplyPassives))

(event Input|KeyboardEvents|1
  (params (Key :type Key%20Structure))
  (:Released
    (bind _returnvalue (Actor|GetActorOfClass "/Game/ThirdPerson/Blueprints/BP_ThirdPersonCharacter.BP_ThirdPersonCharacter_C"))
    (bind _updateddamage (Default|GetUpdatedDamage _returnvalue))
    (Development|PrintString (Utilities|String|ToString(Float) _updateddamage))))

(fn AddtoInventory
  (params (Talisman :type PDA%20Talisman%20Object%20Reference) (Quantity :type Integer))
  (Utilities|Map|Add (Variables|Default|GetTalismanContent) Talisman (+ Quantity (.Value (Utilities|Map|Find (Variables|Default|GetTalismanContent) Talisman)))))

(fn RemovefromInventory
  (params (Talisman :type PDA%20Talisman%20Object%20Reference) (Quantity :type Integer))
  (Utilities|Map|Add (Variables|Default|GetTalismanContent) Talisman (Math|Integer|Max(Integer) (- Quantity (.Value (Utilities|Map|Find (Variables|Default|GetTalismanContent) Talisman))))))

(fn QueryInventory
  (params (Talisman :type PDA%20Talisman%20Object%20Reference))
  (return (.Value (Utilities|Map|Find (Variables|Default|GetTalismanContent) Talisman))))