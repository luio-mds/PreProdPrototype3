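; Actor component that lets one player character signal a request for help to the other player.
; RequestHelpFromOtherPlayer checks whether its owner is the third-person character, then finds the opposite character with GetActorOfClass, assuming one secondary and one third-person character.
; It shows that character's RequestHelpWidget and hides it again after a ten-second delay.
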(event Custom|RequestHelpFromOtherPlayer
  ;[0.15 0.15 0.15 0.5] check which character requested help
  (if (== (Components|GetOwner) "/Game/ThirdPerson/Blueprints/BP_ThirdPersonCharacter.BP_ThirdPersonCharacter")
    (bind _returnvalue (Actor|GetActorOfClass "/Game/ThirdPerson/Blueprints/BP_SecondaryPlayerCharacter.BP_SecondaryPlayerCharacter_C"))
    (Rendering|SetVisibility (Variables|/Game/ThirdPerson/Blueprints/BP_SecondaryPlayerCharacter.BP_SecondaryPlayerCharacter_C|GetRequestHelpWidget _returnvalue) true false)
    (Utilities|FlowControl|Delay 1e+01)
    (Rendering|SetVisibility (Variables|/Game/ThirdPerson/Blueprints/BP_SecondaryPlayerCharacter.BP_SecondaryPlayerCharacter_C|GetRequestHelpWidget _returnvalue) false false)
    (else
      (bind _returnvalue_2 (Actor|GetActorOfClass "/Game/ThirdPerson/Blueprints/BP_ThirdPersonCharacter.BP_ThirdPersonCharacter_C"))
      (Rendering|SetVisibility (Variables|/Game/ThirdPerson/Blueprints/BP_ThirdPersonCharacter.BP_ThirdPersonCharacter_C|GetRequestHelpWidget _returnvalue_2) true false)
      (Utilities|FlowControl|Delay 1e+01)
      (Rendering|SetVisibility (Variables|/Game/ThirdPerson/Blueprints/BP_ThirdPersonCharacter.BP_ThirdPersonCharacter_C|GetRequestHelpWidget _returnvalue_2) false false))))